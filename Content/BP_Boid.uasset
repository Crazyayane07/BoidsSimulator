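; Boid actor for a flocking simulation, holding a velocity that starts in a random direction at a random speed.
; Accelerate adds Acceleration to Velocity unless the sum is NaN; Tick only calls the parent, so steering and movement are not computed here.
; When CanDebugDraw is on, Accelerate prints its state and DebugDraw shows the obstacle separation arrow.
; The alignment, cohesion and separation arrows are disconnected and never run.
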(event EventBeginPlay
  (|CallParentFunction)
  (Variables|Default|SetVelocity (* (Math|Random|RandomUnitVector) (Math|Random|RandomFloatinRange 3.0 5.0))))

(event EventTick
  (params (DeltaSeconds :type Float%20%28single-precision%29))
  (|CallParentFunction DeltaSeconds))

(event EventAccelerate
  (bind _acceleration (Variables|Default|GetAcceleration))
  (if (not (Class|KismetMathLibrary|VectorIsNAN (+ (Variables|Default|GetVelocity) (Variables|Default|GetAcceleration))))
    (Variables|Default|SetVelocity (+ (Variables|Default|GetVelocity) (Variables|Default|GetAcceleration)))
    (if (Variables|Default|GetCanDebugDraw)
      (Development|PrintString (Utilities|String|Append "Velocity:  " (Utilities|String|ToString(Vector) (Variables|Default|GetVelocity)) "  Acceleration:  " (Utilities|String|ToString(Vector) _acceleration) "   Position:   " (Utilities|String|ToString(Vector) (Transformation|GetActorLocation)) "   v + a =  " (Utilities|String|ToString(Vector) (+ (Variables|Default|GetVelocity) _acceleration)))))))

(event EventDebugDraw
  (params (AllignVector :type Vector%20%28by%20ref%29 :default "0, 0, 0") (CohensionVector :type Vector%20%28by%20ref%29 :default "0, 0, 0") (SeparationVector :type Vector%20%28by%20ref%29 :default "0, 0, 0") (SeparationObstacleVector :type Vector%20%28by%20ref%29 :default "0, 0, 0"))
  (bind _returnvalue (Transformation|GetActorLocation))
  (if (Variables|Default|GetCanDebugDraw)
    (Rendering|Debug|DrawDebugArrow _returnvalue (+ _returnvalue SeparationObstacleVector) 5.0 "(R=0.075611,G=0.000000,B=1.000000,A=1.000000)" 1.0 1.0)))

(fn ConstructionScript)