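; Boids manager actor that, in this Blueprint, only supplies random spawn positions; its event graph and construction script are empty.
; GetSpawnPosition picks a random point per axis around the actor's location, using half of the Box component's extent in each direction.
; Points therefore fill only the central half of each box dimension and ignore rotation, scale and any component offset.
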(event EventBeginPlay)

(event Collision|EventActorBeginOverlap
  (params (OtherActor :type Actor%20Object%20Reference)))

(event EventTick
  (params (DeltaSeconds :type Float%20%28single-precision%29)))

(fn ConstructionScript)

(fn GetSpawnPosition
  (bind _returnvalue (Transformation|GetActorLocation))
  (bind _box (Variables|Default|GetBox))
  (bind (_x _y _z) (Math|Vector|BreakVector _returnvalue))
  (bind _boxextent (Variables|/Script/Engine.BoxComponent|GetBoxExtent _box))
  (bind (_x_2 _y_2 _z_2) (Math|Vector|BreakVector _boxextent))
  (bind _returnvalue_2 (/ _z_2 2.0))
  (bind _returnvalue_3 (/ _x_2 2.0))
  (bind _returnvalue_4 (/ _y_2 2.0))
  (return (Math|Vector|MakeVector (Math|Random|RandomFloatinRange (- _x _returnvalue_3) (+ _x _returnvalue_3)) (Math|Random|RandomFloatinRange (- _y _returnvalue_4) (+ _y _returnvalue_4)) (Math|Random|RandomFloatinRange (- _z _returnvalue_2) (+ _z _returnvalue_2)))))